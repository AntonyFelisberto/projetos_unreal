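; BPA_FireBall is a fireball projectile actor that damages the player on contact.
; When its sphere overlaps BP_Player, it stops its particle system, spawns an explosion, sends a hit message with fixed damage crediting the Dragon, and destroys itself.
; An EndOfFireBall event also explodes and removes it after a brief delay, while a BeginPlay timer destroys it silently after a few seconds.
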(event OnComponentBeginOverlap(Sphere)
  (params (OverlappedComponent :type Primitive%20Component%20Object%20Reference) (OtherActor :type Actor%20Object%20Reference) (OtherComp :type Primitive%20Component%20Object%20Reference) (OtherBodyIndex :type Integer) (bFromSweep :type Boolean) (SweepResult :type Hit%20Result%20Structure%20%28by%20ref%29))
  (bind _asbp_player (Utilities|Casting|CastToBP_Player OtherActor))
  (Components|Activation|Deactivate (Variables|Default|GetParticleSystem))
  (Effects|SpawnEmitteratLocation "/Game/StarterContent/Particles/P_Explosion.P_Explosion" (Transformation|GetActorLocation) "0, 0, 0" "2.000000,2.000000,2.000000")
  (Class|BPICombat|INTHitHandle(Message) _asbp_player (Variables|Default|GetDragon) 5.0 (Variables|Default|GetAdditional%20Info))
  (Actor|DestroyActor))

(event Custom|EndOfFireBall
  (Effects|SpawnEmitteratLocation "/Game/StarterContent/Particles/P_Explosion.P_Explosion" (Transformation|GetActorLocation) "0, 0, 0" "2.000000,2.000000,2.000000")
  (Utilities|FlowControl|Delay 0.1)
  (Actor|DestroyActor))

(event EventBeginPlay
  (Utilities|FlowControl|Delay 6.0)
  (Actor|DestroyActor))

(fn ConstructionScript)