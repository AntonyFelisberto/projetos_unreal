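; Game mode for a block-breaking game that tracks remaining blocks and score and handles level clear and restart.
; BeginPlay counts all BP_MyBlock actors, and ReduceBlockCount decrements that count.
; At zero it shows the clear widget and mouse cursor, then after a short delay calls SetGamePaused with false, so the game is not paused.
; AddScore adds a fixed amount, and RESTART reopens the current level.
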(event Custom|RESTART
  (bind _returnvalue (Game|GetCurrentLevelName true))
  (Game|OpenLevel(byName) (Utilities|String|StringToName _returnvalue)))

(event Custom|ReduceBlockCount
  (bind _result (Math|Integer|DecrementInt (Variables|Default|GetBlockCount))
    (:%20%20
      (if (== _result 0)
        (bind _returnvalue (UserInterface|CreateWidget "/Game/BLUEPRINTS/BP_MyGameClearUI.BP_MyGameClearUI_C"))
        (UserInterface|Viewport|AddtoViewport _returnvalue 0)
        (Variables|/Script/Engine.PlayerController|SetbShowMouseCursor (Game|GetPlayerController 0) true)
        (Utilities|FlowControl|Delay 0.2)
        (Game|SetGamePaused false)))))

(event Custom|AddScore
  (Variables|Default|SetScore (+ (Variables|Default|GetScore) 100)))

(event EventBeginPlay
  (bind _outactors (Actor|GetAllActorsOfClass "/Game/BLUEPRINTS/BP_MyBlock.BP_MyBlock_C"))
  (bind _output_get (Variables|Default|SetBlockCount (Utilities|Array|Length _outactors)))
  (Development|PrintString (Utilities|String|ToString(Integer) _output_get)))

(event EventTick
  (params (DeltaSeconds :type Float%20%28single-precision%29)))

(fn ConstructionScript)